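; Guard AI pawn that patrols points, chases pawns it sees and prints "tag" when the player gets close.
; An external playerseen call supplies a destination and patrol points; the guard moves there, walks the points, then returns to its start location.
; PawnSensing triggers a move to the seen pawn's current location, resuming patrol on success or failure, though only success clears Chasing.
; BeginPlay polls player distance until the first tag.
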(event OnSeePawn(PawnSensing)
  (params (Pawn :type Pawn%20Object%20Reference))
  (CallFunction|Chase))

(event Custom|playerseen'
  (params (Destination :type Vector) (patrolpoint :type Array%20of%20Actor%20Object%20References))
  (Variables|Default|Setpatrolpoint patrolpoint)
  (AI|AIMoveTo self Destination 0 5e+01 false
    (:OnSuccess
      (Utilities|FlowControl|Delay 1.0)
      (if (not (Variables|Default|Getchasing))
        (CallFunction|Patrol)))))

(event Custom|returntostart
  (AI|AIMoveTo self (Variables|Default|Getstartlocal) 0 5.0 false))

(event Custom|patrol
  (AI|AIMoveTo self "0, 0, 0" (Utilities|Array|Get(acopy) (Variables|Default|Getpatrolpoint) (Variables|Default|Getindex)) 5e+01 false :!label _label
    (:OnSuccess
      (Utilities|FlowControl|Delay 2.0)
      (Math|Integer|IncrementInt (Variables|Default|Getindex)
        (:%20%20
          (if (not (Variables|Default|Getchasing))
            (if (>= (Variables|Default|Getindex) (Utilities|Array|Length (Variables|Default|Getpatrolpoint)))
              (CallFunction|Returntostart)
              (else
                (goto _label)))))))))

(event Custom|chase
  (Variables|Default|Setchasing true)
  (AI|AIMoveTo self (Transformation|GetActorLocation (stale OnSeePawn(PawnSensing) Pawn)) 0 5e+01 false
    (:OnSuccess
      (Variables|Default|Setchasing false))
    (:OnFail
      _))
  (CallFunction|Patrol))

(event EventBeginPlay
  (Variables|Default|Setstartlocal (Transformation|GetWorldLocation (Variables|Collision|GetCapsuleComponent)))
  (if (<= (Math|Vector|Distance(Vector) (Transformation|GetWorldLocation (Variables|Collision|GetCapsuleComponent)) (Transformation|GetWorldLocation (Variables|/Script/Engine.Character|GetCapsuleComponent (Game|GetPlayerCharacter 0)))) 5e+01) :!label _label
    (Development|PrintString "tag")
    (else
      (Utilities|FlowControl|Delay 0.2)
      (goto _label))))

(fn ConstructionScript)