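; Camera Blueprint that tests detection through AIPerception and PawnSensing, with only debug prints as responses.
; BeginPlay calls Activate on PawnSensing without reset and prints a greeting; seeing a pawn prints another.
; AIPerception updates print on a successful or failed sense, and a success prints again after a one-second delay that rechecks the same stimulus flag.
; Overlap, Tick and construction logic are empty.
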(event OnSeePawn(PawnSensing)
  (params (Pawn :type Pawn%20Object%20Reference))
  (Development|PrintString "hello"))

(event OnTargetPerceptionUpdated(AIPerception)
  (params (Actor :type Actor%20Object%20Reference) (Stimulus :type AI%20Stimulus%20Structure))
  (bind _bsuccessfullysensed (Utilities|Struct|BreakAIStimulus Stimulus))
  (if _bsuccessfullysensed
    (Development|PrintString "freddy")
    (Utilities|FlowControl|Delay 1.0)
    (if _bsuccessfullysensed
      (Development|PrintString "foxie"))
    (else
      (Development|PrintString "bonnie"))))

(event EventBeginPlay
  (Components|Activation|Activate (Variables|Default|GetPawnSensing) false)
  (Development|PrintString "Hello"))

(event Collision|EventActorBeginOverlap
  (params (OtherActor :type Actor%20Object%20Reference)))

(event EventTick
  (params (DeltaSeconds :type Float%20%28single-precision%29)))

(fn ConstructionScript)